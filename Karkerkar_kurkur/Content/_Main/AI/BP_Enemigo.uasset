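; BP_Enemigo is an enemy pawn that chases the first player and takes damage.
; A self-restarting loop waits one second, then runs AI MoveTo toward the player, repeating on success or failure.
; AnyDamage subtracts from clamped health and updates the W_SaludEnemigo widget.
; DestroyActor requires health below zero, which the zero-floor clamp prevents, so that branch never fires.
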(event Custom|PerseguirAlJugador
  (Utilities|FlowControl|Delay 1.0)
  (AI|AIMoveTo self "0, 0, 0" (Game|Player|GetPlayerPawn 0) 5.0 false
    (:OnSuccess
      _)
    (:OnFail
      _))
  (CallFunction|PerseguirAlJugador))

(event EventBeginPlay
  (CallFunction|PerseguirAlJugador))

(event Game|Damage|EventAnyDamage
  (params (Damage :type Float%20%28single-precision%29) (DamageType :type Damage%20Type%20Object%20Reference) (InstigatedBy :type Controller%20Object%20Reference) (DamageCauser :type Actor%20Object%20Reference))
  (bind _output_get (Variables|Default|SetSaludActual (Math|Float|Clamp(Float) (- (Variables|Default|GetSaludActual) Damage) 0.0 (Variables|Default|GetSaludMaxima))))
  (bind _asw_salud_enemigo (Utilities|Casting|CastToW_SaludEnemigo (UserInterface|GetWidget (Variables|Default|GetWidget))))
  (Class|INTHUD|ActualizarSaludHUD(Message) _asw_salud_enemigo (Variables|Default|GetSaludMaxima) (Variables|Default|GetSaludActual))
  (if (< _output_get 0.0)
    (Actor|DestroyActor)))

(fn ConstructionScript)